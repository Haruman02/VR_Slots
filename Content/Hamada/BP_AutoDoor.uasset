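; BP_AutoDoor is a door actor that slides its Cube along relative X with a Timeline.
; Box overlap, a click on the Cube and BeginPlay all feed one toggle, which plays or reverses the Timeline based on OpenOrClose.
; The OpenCheck guard is set on first trigger and never reset here, so BeginPlay normally consumes the only run.
; End overlap is empty, and Timeline completion only sets OpenOrClose true.
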(event OnComponentBeginOverlap(Box)
  (params (OverlappedComponent :type Primitive%20Component%20Object%20Reference) (OtherActor :type Actor%20Object%20Reference) (OtherComp :type Primitive%20Component%20Object%20Reference) (OtherBodyIndex :type Integer) (bFromSweep :type Boolean) (SweepResult :type Hit%20Result%20Structure%20%28by%20ref%29))
  (if (not (Variables|Default|GetOpen_Check))
    (Variables|Default|SetOpen_Check true)
    (if (Variables|Default|GetOpen_Check)
      (if (Variables|Default|GetOpen%20orClose)
        (bind _新規track_1 (Timeline|タイムライン_0 Reverse)
          (:Update
            (Transformation|SetRelativeLocation (Variables|Default|GetCube) (Math|Vector|MakeVector _新規track_1 0.0 0.0) false false))
          (:Finished
            (Variables|Default|SetOpen%20orClose true)))
        (else
          (Timeline|タイムライン_0 Play))))))

(event OnComponentEndOverlap(Box)
  (params (OverlappedComponent :type Primitive%20Component%20Object%20Reference) (OtherActor :type Actor%20Object%20Reference) (OtherComp :type Primitive%20Component%20Object%20Reference) (OtherBodyIndex :type Integer)))

(event OnClicked(Cube)
  (params (TouchedComponent :type Primitive%20Component%20Object%20Reference) (ButtonPressed :type Key%20Structure :default "None"))
  (Input|EnableInput 0)
  (if (not (Variables|Default|GetOpen_Check))
    (Variables|Default|SetOpen_Check true)
    (if (Variables|Default|GetOpen_Check)
      (if (Variables|Default|GetOpen%20orClose)
        (bind _新規track_1 (Timeline|タイムライン_0 Reverse)
          (:Update
            (Transformation|SetRelativeLocation (Variables|Default|GetCube) (Math|Vector|MakeVector _新規track_1 0.0 0.0) false false))
          (:Finished
            (Variables|Default|SetOpen%20orClose true)))
        (else
          (Timeline|タイムライン_0 Play))))))

(event EventBeginPlay
  (if (not (Variables|Default|GetOpen_Check))
    (Variables|Default|SetOpen_Check true)
    (if (Variables|Default|GetOpen_Check)
      (if (Variables|Default|GetOpen%20orClose)
        (bind _新規track_1 (Timeline|タイムライン_0 Reverse)
          (:Update
            (Transformation|SetRelativeLocation (Variables|Default|GetCube) (Math|Vector|MakeVector _新規track_1 0.0 0.0) false false))
          (:Finished
            (Variables|Default|SetOpen%20orClose true)))
        (else
          (Timeline|タイムライン_0 Play))))))

(fn ConstructionScript)