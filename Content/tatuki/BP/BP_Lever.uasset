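; BP_Lever is a VR lever actor that tilts to follow the player's right motion controller.
; Each Tick, while any actor overlaps its Sphere or Capsule, it finds the VRPawn and looks at MotionControllerRight, applying pitch and roll but keeping its current yaw.
; Disconnected leftover logic searches Bp_Box actors tagged Target to store as TargetActor, but never runs.
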(event EventTick
  (params (DeltaSeconds :type Float%20%28single-precision%29))
  (if (> (Utilities|Array|Length (Collision|GetOverlappingActors (Variables|Default|GetSphere) 0 :!class /Script/Engine.PrimitiveComponent)) 0)
    (bind _returnvalue (Actor|GetActorOfClass "/Game/VRTemplate/Blueprints/VRPawn.VRPawn_C" :!label _label))
    (Transformation|SetActorRotation (Math|Rotator|MakeRotator (.Roll (Math|Rotator|BreakRotator (Math|Rotator|FindLookatRotation (Transformation|GetActorLocation) (Transformation|GetWorldLocation (Variables|/Game/VRTemplate/Blueprints/VRPawn.VRPawn_C|GetMotionControllerRight _returnvalue))))) (.Pitch (Math|Rotator|BreakRotator (Math|Rotator|FindLookatRotation (Transformation|GetActorLocation) (Transformation|GetWorldLocation (Variables|/Game/VRTemplate/Blueprints/VRPawn.VRPawn_C|GetMotionControllerRight _returnvalue))))) (.Yaw (Math|Rotator|BreakRotator (Transformation|GetActorRotation)))))
    (elif (> (Utilities|Array|Length (Collision|GetOverlappingActors (Variables|Default|GetCapsule) 0 :!class /Script/Engine.PrimitiveComponent)) 0)
      (goto _label))))

(event Collision|EventActorBeginOverlap
  (params (OtherActor :type Actor%20Object%20Reference)))

(fn ConstructionScript)